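; Large fire hazard actor that burns the puzzle character unless they have a shield.
; Entering the collision box with a shield fades the looping-fire sound, deactivates the fire effects and destroys the actor.
; Without one, it shows a get-the-shield widget, a damage post-process and audio, and starts a looping timer calling the character's TakeDamage by name.
; Leaving the box while burning removes the widget, feedback and timer.
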(event `self.ReceiveBeginPlay`
  ;[1 1 1] Set large fire sound and set take damage indicator to invisible
  (bind _returnvalue (`GameplayStatics.SpawnSoundAtLocation` "/Game/Sounds/Fires/LargeFire_Cue.LargeFire_Cue" (`self.K2_GetActorLocation`) (struct) 1.0 1.0 0.0 null null))
  (set `self.Largefiresound` _returnvalue)
  (set `PostProcessComponent.BlendWeight` 0.0 (`self.PostProcess - take Damage`)))

(event `self.collision box for fire.OnComponentBeginOverlap`
  (params (OverlappedComponent :type "PrimitiveComponent Object Reference") (OtherActor :type "Actor Object Reference") (OtherComp :type "PrimitiveComponent Object Reference") (OtherBodyIndex :type Integer) (bFromSweep :type Boolean) (SweepResult :type "HitResult Structure (by ref)"))
  (bind _aspuzzle_character (cast `/Game/Blueprints/Character/PuzzleCharacter` OtherActor))
  (set `self.ReftoPuzzleCharacter` _aspuzzle_character)
  (if (`/Game/Blueprints/Character/PuzzleCharacter.HasSheild` (`self.ReftoPuzzleCharacter`))
    ;[1 1 1] Fade out fire sound and deactivate fires and then destroy the actor
    (`AudioComponent.FadeOut` (`self.Largefiresound`) 2.5 0.0)
    (`ActorComponent.Deactivate` (`self.LargeFire`))
    (`ActorComponent.Deactivate` (`self.LargeFire1`))
    (`ActorComponent.Deactivate` (`self.LargeFire2`))
    (`ActorComponent.Deactivate` (`self.LargeFire3`))
    (`ActorComponent.Deactivate` (`self.LargeFire4`))
    (`KismetSystemLibrary.Delay` 1.0)
    (`self.K2_DestroyActor`)
    (else
      ;[1 1 1] Post a message to the screen turn on damage indicator soundFX and repeatedly take damage every second
      (set `self.IsBurning` true)
      (bind _returnvalue (`|CreateWidget` "/Game/Blueprints/HUDs/GetTheFireSheild.GetTheFireSheild_C"))
      (`UserWidget.AddToViewport` _returnvalue 0)
      (set `PostProcessComponent.BlendWeight` 1.0 (`self.PostProcess - take Damage`))
      (`ActorComponent.Activate` (`self.Audio`) false)
      (bind _returnvalue_2 (`KismetSystemLibrary.K2_SetTimer` (`self.ReftoPuzzleCharacter`) "TakeDamage" 1.0 true))
      (set `self.DamageTimerHandle` _returnvalue_2))))

(event `self.collision box for fire.OnComponentEndOverlap`
  (params (OverlappedComponent :type "PrimitiveComponent Object Reference") (OtherActor :type "Actor Object Reference") (OtherComp :type "PrimitiveComponent Object Reference") (OtherBodyIndex :type Integer))
  ;[1 1 1] Remove FireSheild Message from screen, turn off Damage indicator, and stop taking damage
  (cast `/Game/Blueprints/Character/PuzzleCharacter` OtherActor)
  (if (`self.IsBurning`)
    (set `self.IsBurning` false)
    (set `PostProcessComponent.BlendWeight` 0.0 (`self.PostProcess - take Damage`))
    (bind _foundwidgets (`WidgetBlueprintLibrary.GetAllWidgetsOfClass` "/Game/Blueprints/HUDs/GetTheFireSheild.GetTheFireSheild_C"))
    (`Widget.RemoveFromParent` _foundwidgets)
    (`ActorComponent.Deactivate` (`self.Audio`))
    (`KismetSystemLibrary.K2_ClearAndInvalidateTimerHandle` (`self.DamageTimerHandle`))))

(fn `UserConstructionScript`)