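; Floor switch that PuzzleCharacters or a BP_BetrayalStatue trigger by overlapping its box, messaging AffectedActors through SwitchInterface.
; The first character in, or a statue, sends activate, plays a sound and moves the mesh vertically on a timeline.
; The last character out sends deactivate and reverses the timeline unless StayActive is set; statue exits are ignored.
; The Activated flag acts as a brief re-trigger guard rather than the pressed state.
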(event `self.ReceiveBeginPlay`
  (set `self.InitialSwitchLocation` (`SceneComponent.K2_GetComponentLocation` (`self.SwitchMesh`))))

(event `self.Box.OnComponentBeginOverlap`
  (params (OverlappedComponent :type "PrimitiveComponent Object Reference") (OtherActor :type "Actor Object Reference") (OtherComp :type "PrimitiveComponent Object Reference") (OtherBodyIndex :type Integer) (bFromSweep :type Boolean) (SweepResult :type "HitResult Structure (by ref)"))
  (bind _characters (`self.Characters`))
  (if (not (`self.Activated`))
    (bind _aspuzzle_character (cast `/Game/Blueprints/Character/PuzzleCharacter` OtherActor)
      (:`then`
        (set `self.Activated` true)
        (`|ExecutionSequence`
          (:`then_0`
            (`KismetSystemLibrary.Delay` 0.2)
            (set `self.Activated` false))
          (:`then_1`
            (`KismetArrayLibrary.Array_Add` _characters _aspuzzle_character)
            (if (== (`KismetArrayLibrary.Array_Length` _characters) 1)
              (set `self.Activated` false :!label _label)
              (for _array_element (`self.AffectedActors`)
                (if (`KismetSystemLibrary.DoesImplementInterface` _array_element "/Game/Blueprints/SwitchInterface.SwitchInterface_C")
                  (message `/Game/Blueprints/SwitchInterface.Activate` _array_element)))
              (`GameplayStatics.PlaySound2D` (`self.SwitchSound`) 1.0 1.0 0.0 null null)
              (bind (_direction _switchelevation) (`Timeline|SwitchTimeline` :!label _label_2)
                (:`Update`
                  (`SceneComponent.K2_SetWorldLocation` (`self.SwitchMesh`) (`KismetMathLibrary.MakeVector` (.x (`self.InitialSwitchLocation`)) (.y (`self.InitialSwitchLocation`)) (+ (.z (`self.InitialSwitchLocation`)) _switchelevation)) false false))
                (:`Finished`
                  (set `self.Activated` false)))))))
      (:`CastFailed`
        (cast `/Game/Blueprints/Actors/BP_BetrayalStatue` OtherActor)
        (set `self.Activated` true)
        (`GameplayStatics.PlaySound2D` (`self.SwitchSound`) 1.0 1.0 0.0 null null)
        (goto _label)))))

(event `self.Box.OnComponentEndOverlap`
  (params (OverlappedComponent :type "PrimitiveComponent Object Reference") (OtherActor :type "Actor Object Reference") (OtherComp :type "PrimitiveComponent Object Reference") (OtherBodyIndex :type Integer))
  (bind _aspuzzle_character (cast `/Game/Blueprints/Character/PuzzleCharacter` OtherActor))
  (if (`self.Activated`)
    _
    (elif (not (`self.StayActive`))
      (`KismetArrayLibrary.Array_RemoveItem` (`self.Characters`) _aspuzzle_character)
      (if (== (`KismetArrayLibrary.Array_Length` (`self.Characters`)) 0)
        (for _array_element (`self.AffectedActors`)
          (if (`KismetSystemLibrary.DoesImplementInterface` _array_element "/Game/Blueprints/SwitchInterface.SwitchInterface_C")
            (message `/Game/Blueprints/SwitchInterface.Deactivate` _array_element)))
        (`GameplayStatics.PlaySound2D` (`self.SwitchSound`) 1.0 1.0 0.0 null null)
        (goto _label_2 :!via `Reverse`)))))

(fn `UserConstructionScript`)