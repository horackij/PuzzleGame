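; Crypt double door actor that swings open when a PuzzleCharacter holding the key enters its box trigger.
; BeginPlay caches both leaves' world rotations, and a timeline adds yaw offsets to them, playing once with a sound.
; Without the key, overlap shows a GetTheKey prompt widget.
; End overlap looks up GetTheKey widgets by class to remove them, rather than storing a reference.
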(event `self.ReceiveBeginPlay`
  ;[1 1 1] Get Door Initial Settings
  (set `self.InitialLeftsideRotation` (`SceneComponent.K2_GetComponentRotation` (`self.LeftSideDoor`)))
  (set `self.InitialRightSideRotation` (`SceneComponent.K2_GetComponentRotation` (`self.RightSideDoor`))))

(event `self.BoxCollision.OnComponentBeginOverlap`
  (params (OverlappedComponent :type "PrimitiveComponent Object Reference") (OtherActor :type "Actor Object Reference") (OtherComp :type "PrimitiveComponent Object Reference") (OtherBodyIndex :type Integer) (bFromSweep :type Boolean) (SweepResult :type "HitResult Structure (by ref)"))
  ;[1 1 1] OpenCrypt Doors
  (bind _aspuzzle_character (cast `/Game/Blueprints/Character/PuzzleCharacter` OtherActor))
  (if (`/Game/Blueprints/Character/PuzzleCharacter.HasKey` _aspuzzle_character)
    (if (not (`self.DoorIsOpen`))
      (`GameplayStatics.PlaySound2D` (`self.DoorSound`) 1.0 1.0 0.0 null null)
      (set `self.DoorIsOpen` true)
      (bind (_direction _leftsidedoor _rightsidedoor) (`Timeline|DoorTimeline`)
        (:`Update`
          (`SceneComponent.K2_SetWorldRotation` (`self.LeftSideDoor`) (`KismetMathLibrary.MakeRotator` (.roll (`self.InitialLeftsideRotation`)) (.pitch (`self.InitialLeftsideRotation`)) (+ (.yaw (`self.InitialLeftsideRotation`)) _leftsidedoor 0.0)) false false)
          (`SceneComponent.K2_SetWorldRotation` (`self.RightSideDoor`) (`KismetMathLibrary.MakeRotator` (.roll (`self.InitialRightSideRotation`)) (.pitch (`self.InitialRightSideRotation`)) (+ (.yaw (`self.InitialRightSideRotation`)) _rightsidedoor 0.0)) false false))))
    (else
      (bind _returnvalue (`|CreateWidget` "/Game/Blueprints/HUDs/GetTheKey.GetTheKey_C"))
      (`UserWidget.AddToViewport` _returnvalue 0))))

(event `self.BoxCollision.OnComponentEndOverlap`
  (params (OverlappedComponent :type "PrimitiveComponent Object Reference") (OtherActor :type "Actor Object Reference") (OtherComp :type "PrimitiveComponent Object Reference") (OtherBodyIndex :type Integer))
  ;[1 1 1] Remove get the key message from screen if it is there
  (bind _foundwidgets (`WidgetBlueprintLibrary.GetAllWidgetsOfClass` "/Game/Blueprints/HUDs/GetTheKey.GetTheKey_C"))
  (`Widget.RemoveFromParent` _foundwidgets))

(fn `UserConstructionScript`)