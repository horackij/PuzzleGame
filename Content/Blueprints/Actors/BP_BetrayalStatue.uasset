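; BP_BetrayalStatue is a statue actor that the puzzle character can push.
; When a PuzzleCharacter enters its Box trigger, the Statue component starts simulating physics and the Audio component plays from the start.
; When that character leaves the trigger, physics simulation turns off and the audio stops, so the statue simulates only during overlap.
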(event `self.Box.OnComponentBeginOverlap`
  (params (OverlappedComponent :type "PrimitiveComponent Object Reference") (OtherActor :type "Actor Object Reference") (OtherComp :type "PrimitiveComponent Object Reference") (OtherBodyIndex :type Integer) (bFromSweep :type Boolean) (SweepResult :type "HitResult Structure (by ref)"))
  ;[1 1 1] Simulate Pushing the Statue
  (cast `/Game/Blueprints/Character/PuzzleCharacter` OtherActor)
  (`PrimitiveComponent.SetSimulatePhysics` (`self.Statue`) true)
  (`AudioComponent.Play` (`self.Audio`) 0.0))

(event `self.Box.OnComponentEndOverlap`
  (params (OverlappedComponent :type "PrimitiveComponent Object Reference") (OtherActor :type "Actor Object Reference") (OtherComp :type "PrimitiveComponent Object Reference") (OtherBodyIndex :type Integer))
  ;[1 1 1] End Simulating Pushing
  (cast `/Game/Blueprints/Character/PuzzleCharacter` OtherActor)
  (`PrimitiveComponent.SetSimulatePhysics` (`self.Statue`) false)
  (`AudioComponent.Stop` (`self.Audio`)))

(fn `UserConstructionScript`)