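; Switch-driven platform actor that raises its Platform component along Z once enough switches are active.
; Activate and Deactivate events adjust a switch counter compared against SwitchRequirement.
; Reaching the requirement plays a sound and runs DoorTimeline, whose elevation track offsets the component from its BeginPlay world location.
; Dropping below the requirement reverses the timeline, unless StayOpen is set.
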(event `self.ReceiveBeginPlay`
  (set `self.InitialDoorLocation` (`SceneComponent.K2_GetComponentLocation` (`self.Platform`))))

(event `/Game/Blueprints/SwitchInterface.Activate`
  (`/Engine/EditorBlueprintResources/StandardMacros.IncrementInt` (`self.SwitchesActivated`)
    (:`  `
      (if (>= (`self.SwitchesActivated`) (`self.SwitchRequirement`))
        (`GameplayStatics.PlaySound2D` (`self.DoorSound`) 1.0 1.0 0.0 null null)
        (bind (_direction _doorelevation) (`Timeline|DoorTimeline` :!label _label)
          (:`Update`
            (`SceneComponent.K2_SetWorldLocation` (`self.Platform`) (`KismetMathLibrary.MakeVector` (.x (`self.InitialDoorLocation`)) (.y (`self.InitialDoorLocation`)) (+ (.z (`self.InitialDoorLocation`)) _doorelevation)) false false)))))))

(event `/Game/Blueprints/SwitchInterface.Deactivate`
  (`/Engine/EditorBlueprintResources/StandardMacros.DecrementInt` (`self.SwitchesActivated`)
    (:`  `
      (if (< (`self.SwitchesActivated`) (`self.SwitchRequirement`))
        (if (not (`self.StayOpen`))
          (goto _label :!via `Reverse`))))))

(fn `UserConstructionScript`)