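; A torch-bearing statue puzzle actor that turns and lights its torch when enough switches are active.
; Activate and Deactivate keep a switch count; reaching the requirement plays a sound and runs a timeline that yaws the statue from its starting rotation.
; Timeline updates also trigger the delayed fire effect and burning sound.
; Dropping below the requirement reverses the timeline unless StayOpen is set, but never extinguishes the fire.
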(event `self.ReceiveBeginPlay`
  (bind _torchfire (`self.TorchFire`))
  ;[1 1 1] Get InitialStatue Locations and rotations/set torch fires to be invisble
  (set `self.InitialDoorLocation` (`SceneComponent.K2_GetComponentLocation` (`self.Statue`)))
  (set `self.InitialRotation` (`SceneComponent.K2_GetComponentRotation` (`self.Statue`)))
  (`SceneComponent.SetVisibility` _torchfire false false)
  (`ActorComponent.Deactivate` _torchfire))

(event `/Game/Blueprints/SwitchInterface.Activate`
  ;[1 1 1] What happens when stepping on all required switches
  (`/Engine/EditorBlueprintResources/StandardMacros.IncrementInt` (`self.SwitchesActivated`)
    (:`  `
      (if (>= (`self.SwitchesActivated`) (`self.SwitchRequirement`))
        (`GameplayStatics.PlaySound2D` (`self.DoorSound`) 1.0 1.0 0.0 null null)
        ;[1 1 1] Rotate the statues and ignite the tourches
        (bind (_direction _statuerotation) (`Timeline|DoorTimeline` :!label _label)
          (:`Update`
            (`SceneComponent.K2_SetWorldRotation` (`self.Statue`) (`KismetMathLibrary.MakeRotator` (.roll (`self.InitialRotation`)) (.pitch (`self.InitialRotation`)) (+ (.yaw (`self.InitialRotation`)) _statuerotation)) false false)
            (`KismetSystemLibrary.Delay` 1.0)
            (`SceneComponent.SetVisibility` (`self.TorchFire`) true false)
            (`ActorComponent.Activate` (`self.TorchFire`) false)
            (`KismetSystemLibrary.Delay` 0.2)
            (`GameplayStatics.PlaySoundAtLocation` "/Game/Sounds/Fires/TorchBurning_Cue.TorchBurning_Cue" (`self.K2_GetActorLocation`) (struct) 1.0 1.0 0.0 null null null)))))))

(event `/Game/Blueprints/SwitchInterface.Deactivate`
  ;[1 1 1] What happens when stepping off the required switches
  (`/Engine/EditorBlueprintResources/StandardMacros.DecrementInt` (`self.SwitchesActivated`)
    (:`  `
      (if (< (`self.SwitchesActivated`) (`self.SwitchRequirement`))
        (if (not (`self.StayOpen`))
          (goto _label :!via `Reverse`))))))

(fn `UserConstructionScript`)