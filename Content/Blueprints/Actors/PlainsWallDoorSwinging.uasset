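; A swinging wall door that opens once enough switches are active.
; Activate and Deactivate adjust a switch count that is compared against SwitchRequirement; dropping below it closes the door unless StayOpen is set.
; A timeline adds yaw to the rotation saved at BeginPlay, playing forward to open and reversing to close, with a 2D sound.
; Only opening checks DoorIsOpen, so the close sound can replay on an already closed door.
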(event `self.ReceiveBeginPlay`
  (set `self.InitialDoorLocation` (`SceneComponent.K2_GetComponentLocation` (`self.DoorMesh`)))
  (set `self.InitialDoorRotation` (`SceneComponent.K2_GetComponentRotation` (`self.DoorMesh`))))

(event `/Game/Blueprints/SwitchInterface.Activate`
  (`/Engine/EditorBlueprintResources/StandardMacros.IncrementInt` (`self.SwitchesActivated`)
    (:`  `
      (if (>= (`self.SwitchesActivated`) (`self.SwitchRequirement`))
        (if (not (`self.DoorIsOpen`))
          (`GameplayStatics.PlaySound2D` (`self.DoorSound`) 1.0 1.0 0.0 null null)
          (set `self.DoorIsOpen` true)
          (bind (_direction _doorrotation) (`Timeline|DoorTimeline` :!label _label)
            (:`Update`
              (`SceneComponent.K2_SetWorldRotation` (`self.DoorMesh`) (`KismetMathLibrary.MakeRotator` (.roll (`self.InitialDoorRotation`)) (.pitch (`self.InitialDoorRotation`)) (+ (.yaw (`self.InitialDoorRotation`)) _doorrotation)) false false))))))))

(event `/Game/Blueprints/SwitchInterface.Deactivate`
  (`/Engine/EditorBlueprintResources/StandardMacros.DecrementInt` (`self.SwitchesActivated`)
    (:`  `
      (if (< (`self.SwitchesActivated`) (`self.SwitchRequirement`))
        (if (not (`self.StayOpen`))
          (`GameplayStatics.PlaySound2D` (`self.DoorSound`) 1.0 1.0 0.0 null null)
          (set `self.DoorIsOpen` false)
          (goto _label :!via `Reverse`))))))

(fn `UserConstructionScript`)